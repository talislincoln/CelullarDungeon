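; BP_DictionaryIntTriangleList is a dictionary that maps an integer vertex index to a list of triangles.
; It stores parallel Keys and Values arrays, with each value being a BP_TriangleList object that wraps its own array.
; AddTriangle appends to an existing key's list or constructs a new wrapper for a new key.
; GetValues looks up the list by index without checking that the key exists.
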(fn Clear
  (Utilities|Array|Clear (Variables|Default|GetKeys))
  (Utilities|Array|Clear (Variables|Default|GetValues)))

(fn ContainsKey
  (params (Key :type Integer))
  (return (Utilities|Array|ContainsItem (Variables|Default|GetKeys) Key)))

(fn AddTriangle
  (params (VertexIndexKey :type Integer) (Triangle :type BP%20Triangle%20Object%20Reference))
  (bind _keys (Variables|Default|GetKeys))
  (bind _returnvalue (Utilities|Array|FindItem _keys VertexIndexKey))
  (if (>= _returnvalue 0)
    (Utilities|Array|Add (Variables|/Game/Blueprints/Structures/BP_TriangleList.BP_TriangleList_C|GetTriangleList (Utilities|Array|Get(acopy) (Variables|Default|GetValues) _returnvalue)) Triangle)
    (else
      (Utilities|Array|Add (Variables|Default|GetKeys) VertexIndexKey)
      (bind _returnvalue_2 (Game|ConstructObjectfromClass "/Game/Blueprints/Structures/BP_TriangleList.BP_TriangleList_C" self))
      (Utilities|Array|Add (Variables|/Game/Blueprints/Structures/BP_TriangleList.BP_TriangleList_C|GetTriangleList _returnvalue_2) Triangle)
      (Utilities|Array|Add (Variables|Default|GetValues) _returnvalue_2))))

(fn GetValues
  (params (VertexIndex :type Integer))
  (return (Variables|/Game/Blueprints/Structures/BP_TriangleList.BP_TriangleList_C|GetTriangleList (Utilities|Array|Get(acopy) (Variables|Default|GetValues) (Utilities|Array|FindItem (Variables|Default|GetKeys) VertexIndex)))))