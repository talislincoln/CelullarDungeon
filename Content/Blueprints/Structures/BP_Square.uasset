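; BP_Square is one grid cell built from four corner nodes, laid out as in marching squares.
; Init stores the corners and derives the four edge midpoints from the Right and Above links of the corner nodes.
; It packs the corners' Active flags into a four-bit Configuration index, with top-left as the highest bit, then returns itself.
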(fn Init
  (params (TopLeft :type BP%20Control%20Node%20Object%20Reference) (TopRight :type BP%20Control%20Node%20Object%20Reference) (BottomRight :type BP%20Control%20Node%20Object%20Reference) (BottomLeft :type BP%20Control%20Node%20Object%20Reference))
  (bind _output_get (Variables|Default|SetTopLeft TopLeft))
  (Variables|Default|SetTopRight TopRight)
  (bind _output_get_2 (Variables|Default|SetBottomRight BottomRight))
  (bind _output_get_3 (Variables|Default|SetBottomLeft BottomLeft))
  (Variables|Default|SetCentreTop (Variables|/Game/Blueprints/Structures/BP_ControlNode.BP_ControlNode_C|GetRight _output_get))
  (Variables|Default|SetCentreRight (Variables|/Game/Blueprints/Structures/BP_ControlNode.BP_ControlNode_C|GetAbove _output_get_2))
  (Variables|Default|SetCentreBottom (Variables|/Game/Blueprints/Structures/BP_ControlNode.BP_ControlNode_C|GetRight _output_get_3))
  (Variables|Default|SetCentreLeft (Variables|/Game/Blueprints/Structures/BP_ControlNode.BP_ControlNode_C|GetAbove _output_get_3))
  (Variables|Default|SetConfiguration 0)
  (if (Variables|/Game/Blueprints/Structures/BP_ControlNode.BP_ControlNode_C|GetActive (Variables|Default|GetTopLeft))
    (Variables|Default|SetConfiguration (+ (Variables|Default|GetConfiguration) 8)))
  (if (Variables|/Game/Blueprints/Structures/BP_ControlNode.BP_ControlNode_C|GetActive (Variables|Default|GetTopRight))
    (Variables|Default|SetConfiguration (+ (Variables|Default|GetConfiguration) 4)))
  (if (Variables|/Game/Blueprints/Structures/BP_ControlNode.BP_ControlNode_C|GetActive (Variables|Default|GetBottomRight))
    (Variables|Default|SetConfiguration (+ (Variables|Default|GetConfiguration) 2)))
  (if (Variables|/Game/Blueprints/Structures/BP_ControlNode.BP_ControlNode_C|GetActive (Variables|Default|GetBottomLeft))
    (Variables|Default|SetConfiguration (+ (Variables|Default|GetConfiguration) 1)))
  (return self))