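; BP_ControlNode is a corner node in a square grid, holding a position and an active flag, in a layout resembling marching squares.
; InitControlNode stores both values, then constructs two child BP_Node objects, Above and Right, each offset half a square along +Z and +X respectively.
; It returns itself, and the offsets place the grid in the XZ plane.
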(fn InitControlNode
  (params (Position :type Vector) (Active :type Boolean) (SquareSize :type Integer))
  (bind _returnvalue (/ SquareSize 2))
  (bind _self self)
  (bind _output_get (Variables|Default|SetPosition Position))
  (Variables|Default|SetActive Active)
  (bind _returnvalue_2 (Game|ConstructObjectfromClass "/Game/Blueprints/Structures/BP_Node.BP_Node_C" _self))
  (bind _output_get_2 (Variables|Default|SetAbove _returnvalue_2))
  (Default|Init _output_get_2 (+ _output_get (* "0, 0,1.000000" _returnvalue)))
  (bind _returnvalue_3 (Game|ConstructObjectfromClass "/Game/Blueprints/Structures/BP_Node.BP_Node_C" _self))
  (bind _output_get_3 (Variables|Default|SetRight _returnvalue_3))
  (Default|Init _output_get_3 (+ _output_get (* "1.000000, 0,0.000000" _returnvalue)))
  (return self))