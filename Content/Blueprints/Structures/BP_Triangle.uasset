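; BP_Triangle is a Blueprint data structure that represents one triangle as three vertex indices.
; Init stores the indices both as named A, B, C variables and in a three-element Vertices array, then returns itself so the call can be chained.
; GetVertex reads the array by position, while Contains tests a given vertex index against the three named variables.
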(fn GetVertex
  (params (Index :type Integer))
  (return (Utilities|Array|Get(acopy) (Variables|Default|GetVertices) Index)))

(fn Init
  (params (A :type Integer) (B :type Integer) (C :type Integer))
  (bind _vertices (Variables|Default|GetVertices))
  (bind _output_get (Variables|Default|SetVertexIndexA A))
  (bind _output_get_2 (Variables|Default|SetVertexIndexB B))
  (bind _output_get_3 (Variables|Default|SetVertexIndexC C))
  (Utilities|Array|Resize (Variables|Default|GetVertices) 3)
  (Utilities|Array|SetArrayElem _vertices 0 _output_get)
  (Utilities|Array|SetArrayElem _vertices 1 _output_get_2)
  (Utilities|Array|SetArrayElem _vertices 2 _output_get_3)
  (return self))

(fn Contains
  (params (VertexIndex :type Integer))
  (return (Math|Boolean|ORBoolean (== VertexIndex (Variables|Default|GetVertexIndexA)) (== VertexIndex (Variables|Default|GetVertexIndexB)) (== VertexIndex (Variables|Default|GetVertexIndexC)))))