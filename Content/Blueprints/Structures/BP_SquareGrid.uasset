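; BP_SquareGrid turns a 2D map matrix into a grid of squares with shared corner nodes, in the layout used by marching squares.
; Init creates a BP_ControlNode per map cell, centred around the origin on the XZ plane and active where the cell equals 1.
; It then builds one BP_Square from each 2x2 block of neighbouring nodes, storing nodes and squares in matrix objects.
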(fn Init
  (params (Map :type BP%20Int%20Matrix%20Object%20Reference) (SquareSize :type Integer))
  ;[1 1 1] Init local variables
  (LocalVariables|SetLocalMap Map)
  (LocalVariables|SetLocalSquareSize SquareSize)
  (bind _output_get (Variables|Default|SetNodeCountX (Default|GetNumRows (LocalVariables|GetLocalMap))))
  (Variables|Default|SetMapWidth (* _output_get (LocalVariables|GetLocalSquareSize)))
  (bind _output_get_2 (Variables|Default|SetNodeCountY (Default|GetNumCols (LocalVariables|GetLocalMap))))
  (Variables|Default|SetMapHeight (* _output_get_2 (LocalVariables|GetLocalSquareSize)))
  (bind _returnvalue (Game|ConstructObjectfromClass "/Game/Blueprints/Structures/BP_ControlNodeMatrix.BP_ControlNodeMatrix_C" self))
  (bind _output_get_3 (LocalVariables|SetControlNodes _returnvalue))
  (Default|Init _output_get_3 (Variables|Default|GetNodeCountX) (Variables|Default|GetNodeCountY))
  ;[1 1 1] Create control nodes
  (for _index (range 0 (- (Variables|Default|GetNodeCountX) 1))
    (LocalVariables|SetX _index)
    (for _index_2 (range 0 (- (Variables|Default|GetNodeCountY) 1))
      (LocalVariables|SetY _index_2)
      (bind _returnvalue_2 (Game|ConstructObjectfromClass "/Game/Blueprints/Structures/BP_ControlNode.BP_ControlNode_C" self))
      (bind _controlnode (Default|InitControlNode _returnvalue_2 (Math|Vector|MakeVector (Math|Conversions|ToFloat(Integer) (+ (/ (Variables|Default|GetMapWidth) -2) (* (LocalVariables|GetX) (LocalVariables|GetLocalSquareSize)) (/ (LocalVariables|GetLocalSquareSize) 2))) 0.0 (Math|Conversions|ToFloat(Integer) (+ (/ (LocalVariables|GetLocalSquareSize) 2) (/ (Variables|Default|GetMapHeight) -2) (* (LocalVariables|GetY) (LocalVariables|GetLocalSquareSize))))) (== (Default|GetElement (LocalVariables|GetLocalMap) (LocalVariables|GetX) (LocalVariables|GetY)) 1) (LocalVariables|GetLocalSquareSize)))
      (Default|SetElement (LocalVariables|GetControlNodes) (LocalVariables|GetX) (LocalVariables|GetY) _controlnode)))
  ;[1 1 1] Create a square of control nodes
  (bind _returnvalue_3 (Game|ConstructObjectfromClass "/Game/Blueprints/Structures/BP_SquareMatrix.BP_SquareMatrix_C" self))
  (bind _output_get_4 (Variables|Default|SetSquares _returnvalue_3))
  (Default|Init _output_get_4 (- (Variables|Default|GetNodeCountX) 1) (- (Variables|Default|GetNodeCountY) 1))
  (for _index_3 (range 0 (- (- (Variables|Default|GetNodeCountX) 1) 1))
    (LocalVariables|SetX _index_3)
    (for _index_4 (range 0 (- (- (Variables|Default|GetNodeCountY) 1) 1))
      (LocalVariables|SetY _index_4)
      (bind _returnvalue_4 (Game|ConstructObjectfromClass "/Game/Blueprints/Structures/BP_Square.BP_Square_C" self))
      (bind _square (Default|Init _returnvalue_4 (Default|GetElement (LocalVariables|GetControlNodes) (LocalVariables|GetX) (+ (LocalVariables|GetY) 1)) (Default|GetElement (LocalVariables|GetControlNodes) (+ (LocalVariables|GetX) 1) (+ (LocalVariables|GetY) 1)) (Default|GetElement (LocalVariables|GetControlNodes) (+ (LocalVariables|GetX) 1) (LocalVariables|GetY)) (Default|GetElement (LocalVariables|GetControlNodes) (LocalVariables|GetX) (LocalVariables|GetY))))
      (Default|SetElement (Variables|Default|GetSquares) (LocalVariables|GetX) (LocalVariables|GetY) _square))))