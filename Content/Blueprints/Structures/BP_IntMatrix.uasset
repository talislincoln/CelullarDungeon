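; BP_IntMatrix is a two-dimensional integer matrix object for Blueprint use.
; It stores an array of BP_IntList objects, each wrapping an int array, to work around the lack of nested arrays.
; Init sizes and constructs the rows and returns itself, with Width as the row count and Height as the column count.
; Accessors read rows, read and write elements, and report dimensions, taking column count from the first row.
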(fn Init
  (params (Width :type Integer) (Height :type Integer))
  (bind _data (Variables|Default|GetData))
  (Utilities|Array|Resize _data Width)
  (for (_ _array_index) _data
    (bind _returnvalue (Game|ConstructObjectfromClass "/Game/Blueprints/Structures/BP_IntList.BP_IntList_C" self))
    (Utilities|Array|Resize (Variables|/Game/Blueprints/Structures/BP_IntList.BP_IntList_C|GetIntList _returnvalue) Height)
    (Utilities|Array|SetArrayElem (Variables|Default|GetData) _array_index _returnvalue))
  (return self))

(fn GetRow
  (params (Row :type Integer))
  (return (Variables|/Game/Blueprints/Structures/BP_IntList.BP_IntList_C|GetIntList (Utilities|Array|Get(acopy) (Variables|Default|GetData) Row))))

(fn GetElement
  (params (Row :type Integer) (Column :type Integer))
  (return (Utilities|Array|Get(acopy) (Variables|/Game/Blueprints/Structures/BP_IntList.BP_IntList_C|GetIntList (Utilities|Array|Get(acopy) (Variables|Default|GetData) Row)) Column)))

(fn SetElement
  (params (Row :type Integer) (Column :type Integer) (Value :type Integer))
  (Utilities|Array|SetArrayElem (Variables|/Game/Blueprints/Structures/BP_IntList.BP_IntList_C|GetIntList (Utilities|Array|Get(acopy) (Variables|Default|GetData) Row)) Column Value))

(fn GetNumRows
  (return (Utilities|Array|Length (Variables|Default|GetData))))

(fn GetNumCols
  (return (Utilities|Array|Length (Variables|/Game/Blueprints/Structures/BP_IntList.BP_IntList_C|GetIntList (Utilities|Array|Get(acopy) (Variables|Default|GetData))))))