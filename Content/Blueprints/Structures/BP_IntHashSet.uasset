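; BP_IntHashSet is a helper structure that holds a collection of unique integers.
; It wraps IntList with Add, Contains and Clear functions, with no function for removing a single item.
; Add checks Contains on the list before inserting, so uniqueness comes from that lookup rather than any hashing logic in the Blueprint.
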(fn Add
  (params (Item :type Integer))
  (bind _intlist (Variables|Default|GetIntList))
  (if (not (Utilities|Array|ContainsItem _intlist Item))
    (Utilities|Array|Add _intlist Item)))

(fn Contains
  (params (Item :type Integer))
  (return (Utilities|Array|ContainsItem (Variables|Default|GetIntList) Item)))

(fn Clear
  (Utilities|Array|Clear (Variables|Default|GetIntList)))