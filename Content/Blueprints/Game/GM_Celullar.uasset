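; GM_Celullar is a game mode Blueprint that starts dungeon map generation at BeginPlay.
; It takes the first BP_DungeonGenerator in the level and creates a time-seeded random stream.
; When the generator's GenerateRandomMap is off, it reseeds that stream with the generator's Seed and passes it to the generator.
; It then calls GenerateMap on the generator, whichever seed mode is set.
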(event EventBeginPlay
  (Utilities|FlowControl|Sequence
    (:then_0
      ;[1 1 1] Look for the Dungeon Information
      (bind _outactors (Actor|GetAllActorsOfClass "/Game/Blueprints/Game/BP_DungeonGenerator.BP_DungeonGenerator_C"))
      (Variables|Default|SetDungeonGeneratorActor (Utilities|Array|Get(acopy) _outactors))
      (Variables|Default|SetDungeonDataFound true))
    (:then_1
      ;[1 1 1] Setting Random Seed
      (if (Variables|Default|GetDungeonDataFound)
        (Variables|Default|SetRandomStream (Math|Random|MakeRandomStream (.Seconds (Class|GameplayStatics|GetAccurateRealTime))))
        (if (not (Variables|/Game/Blueprints/Game/BP_DungeonGenerator.BP_DungeonGenerator_C|GetGenerateRandomMap (Variables|Default|GetDungeonGeneratorActor)))
          (Math|Random|SetRandomStreamSeed (Variables|Default|GetRandomStream) (Variables|/Game/Blueprints/Game/BP_DungeonGenerator.BP_DungeonGenerator_C|GetSeed (Variables|Default|GetDungeonGeneratorActor)))
          (Variables|/Game/Blueprints/Game/BP_DungeonGenerator.BP_DungeonGenerator_C|SetRandomStream (Variables|Default|GetDungeonGeneratorActor) (Variables|Default|GetRandomStream)))))
    (:then_2
      (if (Variables|Default|GetDungeonDataFound)
        (Default|GenerateMap (Variables|Default|GetDungeonGeneratorActor))))))

(fn ConstructionScript)