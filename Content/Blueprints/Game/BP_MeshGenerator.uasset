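; Procedural mesh generator that turns a map into a flat surface mesh plus extruded walls using marching squares.
; GenerateMesh builds a square grid from the map and triangulates each square by its configuration, recording triangles per vertex in a dictionary.
; Edges belonging to only one triangle are chained recursively into closed outlines, skipping vertices already checked.
; CreateWallMesh extrudes those outlines down the Y axis by WallHeight into a separate wall mesh.
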(fn ConstructionScript)

(fn GenerateMesh
  (params (Map :type BP%20Int%20Matrix%20Object%20Reference) (SquareSize :type Integer))
  (bind _self self)
  (LocalVariables|SetLocalMap Map)
  (LocalVariables|SetLocalSquareSize SquareSize)
  (bind _returnvalue (Game|ConstructObjectfromClass "/Game/Blueprints/Structures/BP_DictionaryIntTriangleList.BP_DictionaryIntTriangleList_C" _self))
  (bind _output_get (Variables|Default|SetTriangleDictionary _returnvalue))
  (Default|Clear _output_get)
  (bind _returnvalue_2 (Game|ConstructObjectfromClass "/Game/Blueprints/Structures/BP_IntMatrix.BP_IntMatrix_C" _self))
  (bind _output_get_2 (Variables|Default|SetOutlines _returnvalue_2))
  (Default|Init _output_get_2 1 1)
  (Utilities|Array|Clear (Variables|Default|GetCheckedVertices))
  (Utilities|Array|Clear (Variables|Default|GetVertices))
  (Utilities|Array|Clear (Variables|Default|GetTriangles))
  (bind _returnvalue_3 (Game|ConstructObjectfromClass "/Game/Blueprints/Structures/BP_SquareGrid.BP_SquareGrid_C" self))
  (bind _output_get_3 (Variables|Default|SetSquareGrid _returnvalue_3))
  (Default|Init _output_get_3 (LocalVariables|GetLocalMap) (LocalVariables|GetLocalSquareSize))
  (for _index (range 0 (- (Default|GetNumRows (Variables|/Game/Blueprints/Structures/BP_SquareGrid.BP_SquareGrid_C|GetSquares (Variables|Default|GetSquareGrid))) 1))
    (LocalVariables|SetX _index)
    (for _index_2 (range 0 (- (Default|GetNumCols (Variables|/Game/Blueprints/Structures/BP_SquareGrid.BP_SquareGrid_C|GetSquares (Variables|Default|GetSquareGrid))) 1))
      (bind _output_get_4 (LocalVariables|SetY _index_2))
      (CallFunction|TriangulateSquare (Default|GetElement (Variables|/Game/Blueprints/Structures/BP_SquareGrid.BP_SquareGrid_C|GetSquares (Variables|Default|GetSquareGrid)) (LocalVariables|GetX) _output_get_4))))
  (Class|ProceduralMeshComponent|CreateMeshSectionLinearColor (Variables|Default|GetMesh) 0 (Variables|Default|GetVertices) (Variables|Default|GetTriangles) 0 0 0 0 false)
  (CallFunction|CreateWallMesh))

(fn CreateTriangle
  (params (A :type BP%20Node%20Object%20Reference) (B :type BP%20Node%20Object%20Reference) (C :type BP%20Node%20Object%20Reference))
  (bind _vertexindex (Variables|/Game/Blueprints/Structures/BP_Node.BP_Node_C|GetVertexIndex A))
  (bind _vertexindex_2 (Variables|/Game/Blueprints/Structures/BP_Node.BP_Node_C|GetVertexIndex B))
  (bind _triangledictionary (Variables|Default|GetTriangleDictionary))
  (bind _vertexindex_3 (Variables|/Game/Blueprints/Structures/BP_Node.BP_Node_C|GetVertexIndex C))
  (bind _triangles (Variables|Default|GetTriangles))
  (Utilities|Array|Add _triangles _vertexindex)
  (Utilities|Array|Add _triangles _vertexindex_2)
  (Utilities|Array|Add _triangles _vertexindex_3)
  (bind _returnvalue (Game|ConstructObjectfromClass "/Game/Blueprints/Structures/BP_Triangle.BP_Triangle_C" self))
  (bind _triangle (Default|Init _returnvalue _vertexindex _vertexindex_2 _vertexindex_3))
  (Default|AddTriangle _triangledictionary (Variables|/Game/Blueprints/Structures/BP_Triangle.BP_Triangle_C|GetVertexIndexA _triangle) _triangle)
  (Default|AddTriangle _triangledictionary (Variables|/Game/Blueprints/Structures/BP_Triangle.BP_Triangle_C|GetVertexIndexB _triangle) _triangle)
  (Default|AddTriangle _triangledictionary (Variables|/Game/Blueprints/Structures/BP_Triangle.BP_Triangle_C|GetVertexIndexC _triangle) _triangle))

(fn AssignVertices
  (params (Points :type Array%20of%20BP%20Node%20Object%20References))
  (for _array_element Points
    (if (== (Variables|/Game/Blueprints/Structures/BP_Node.BP_Node_C|GetVertexIndex _array_element) -1)
      (Variables|/Game/Blueprints/Structures/BP_Node.BP_Node_C|SetVertexIndex _array_element (Utilities|Array|Length (Variables|Default|GetVertices)))
      (Utilities|Array|Add (Variables|Default|GetVertices) (Variables|/Game/Blueprints/Structures/BP_Node.BP_Node_C|GetPosition _array_element)))))

(fn MeshfromPoints
  (params (Points :type Array%20of%20BP%20Node%20Object%20References))
  (bind _output_get (LocalVariables|SetLocalPoints Points))
  (CallFunction|AssignVertices _output_get)
  (if (>= (Utilities|Array|Length (LocalVariables|GetLocalPoints)) 3)
    (CallFunction|CreateTriangle (Utilities|Array|Get(acopy) (LocalVariables|GetLocalPoints)) (Utilities|Array|Get(acopy) (LocalVariables|GetLocalPoints) 1) (Utilities|Array|Get(acopy) (LocalVariables|GetLocalPoints) 2)))
  (if (>= (Utilities|Array|Length (LocalVariables|GetLocalPoints)) 4)
    (CallFunction|CreateTriangle (Utilities|Array|Get(acopy) (LocalVariables|GetLocalPoints)) (Utilities|Array|Get(acopy) (LocalVariables|GetLocalPoints) 2) (Utilities|Array|Get(acopy) (LocalVariables|GetLocalPoints) 3)))
  (if (>= (Utilities|Array|Length (LocalVariables|GetLocalPoints)) 5)
    (CallFunction|CreateTriangle (Utilities|Array|Get(acopy) (LocalVariables|GetLocalPoints)) (Utilities|Array|Get(acopy) (LocalVariables|GetLocalPoints) 3) (Utilities|Array|Get(acopy) (LocalVariables|GetLocalPoints) 4)))
  (if (>= (Utilities|Array|Length (LocalVariables|GetLocalPoints)) 6)
    (CallFunction|CreateTriangle (Utilities|Array|Get(acopy) (LocalVariables|GetLocalPoints)) (Utilities|Array|Get(acopy) (LocalVariables|GetLocalPoints) 4) (Utilities|Array|Get(acopy) (LocalVariables|GetLocalPoints) 5))))

(fn TriangulateSquare
  (params (Square :type BP%20Square%20Object%20Reference))
  (bind _checkedvertices (Variables|Default|GetCheckedVertices))
  (bind _output_get (LocalVariables|SetLocalSquare Square))
  (switch int (Variables|/Game/Blueprints/Structures/BP_Square.BP_Square_C|GetConfiguration _output_get)
    (:1
      ;[1 1 1] Case 1
      (CallFunction|MeshfromPoints (Utilities|Array|MakeArray (Variables|/Game/Blueprints/Structures/BP_Square.BP_Square_C|GetCentreLeft (LocalVariables|GetLocalSquare)) (Variables|/Game/Blueprints/Structures/BP_Square.BP_Square_C|GetCentreBottom (LocalVariables|GetLocalSquare)) (Variables|/Game/Blueprints/Structures/BP_Square.BP_Square_C|GetBottomLeft (LocalVariables|GetLocalSquare)))))
    (:2
      ;[1 1 1] Case 2
      (CallFunction|MeshfromPoints (Utilities|Array|MakeArray (Variables|/Game/Blueprints/Structures/BP_Square.BP_Square_C|GetBottomRight (LocalVariables|GetLocalSquare)) (Variables|/Game/Blueprints/Structures/BP_Square.BP_Square_C|GetCentreBottom (LocalVariables|GetLocalSquare)) (Variables|/Game/Blueprints/Structures/BP_Square.BP_Square_C|GetCentreRight (LocalVariables|GetLocalSquare)))))
    (:3
      ;[1 1 1] Case 3
      (CallFunction|MeshfromPoints (Utilities|Array|MakeArray (Variables|/Game/Blueprints/Structures/BP_Square.BP_Square_C|GetCentreRight (LocalVariables|GetLocalSquare)) (Variables|/Game/Blueprints/Structures/BP_Square.BP_Square_C|GetBottomRight (LocalVariables|GetLocalSquare)) (Variables|/Game/Blueprints/Structures/BP_Square.BP_Square_C|GetBottomLeft (LocalVariables|GetLocalSquare)) (Variables|/Game/Blueprints/Structures/BP_Square.BP_Square_C|GetCentreLeft (LocalVariables|GetLocalSquare)))))
    (:4
      ;[1 1 1] Case 4
      (CallFunction|MeshfromPoints (Utilities|Array|MakeArray (Variables|/Game/Blueprints/Structures/BP_Square.BP_Square_C|GetTopRight (LocalVariables|GetLocalSquare)) (Variables|/Game/Blueprints/Structures/BP_Square.BP_Square_C|GetCentreRight (LocalVariables|GetLocalSquare)) (Variables|/Game/Blueprints/Structures/BP_Square.BP_Square_C|GetCentreTop (LocalVariables|GetLocalSquare)))))
    (:5
      ;[1 1 1] Case 5
      (CallFunction|MeshfromPoints (Utilities|Array|MakeArray (Variables|/Game/Blueprints/Structures/BP_Square.BP_Square_C|GetCentreTop (LocalVariables|GetLocalSquare)) (Variables|/Game/Blueprints/Structures/BP_Square.BP_Square_C|GetTopRight (LocalVariables|GetLocalSquare)) (Variables|/Game/Blueprints/Structures/BP_Square.BP_Square_C|GetCentreRight (LocalVariables|GetLocalSquare)) (Variables|/Game/Blueprints/Structures/BP_Square.BP_Square_C|GetCentreBottom (LocalVariables|GetLocalSquare)) (Variables|/Game/Blueprints/Structures/BP_Square.BP_Square_C|GetBottomLeft (LocalVariables|GetLocalSquare)) (Variables|/Game/Blueprints/Structures/BP_Square.BP_Square_C|GetCentreLeft (LocalVariables|GetLocalSquare)))))
    (:6
      ;[1 1 1] Case 6
      (CallFunction|MeshfromPoints (Utilities|Array|MakeArray (Variables|/Game/Blueprints/Structures/BP_Square.BP_Square_C|GetCentreTop (LocalVariables|GetLocalSquare)) (Variables|/Game/Blueprints/Structures/BP_Square.BP_Square_C|GetTopRight (LocalVariables|GetLocalSquare)) (Variables|/Game/Blueprints/Structures/BP_Square.BP_Square_C|GetBottomRight (LocalVariables|GetLocalSquare)) (Variables|/Game/Blueprints/Structures/BP_Square.BP_Square_C|GetCentreBottom (LocalVariables|GetLocalSquare)))))
    (:7
      ;[1 1 1] Case 7
      (CallFunction|MeshfromPoints (Utilities|Array|MakeArray (Variables|/Game/Blueprints/Structures/BP_Square.BP_Square_C|GetCentreTop (LocalVariables|GetLocalSquare)) (Variables|/Game/Blueprints/Structures/BP_Square.BP_Square_C|GetTopRight (LocalVariables|GetLocalSquare)) (Variables|/Game/Blueprints/Structures/BP_Square.BP_Square_C|GetBottomRight (LocalVariables|GetLocalSquare)) (Variables|/Game/Blueprints/Structures/BP_Square.BP_Square_C|GetBottomLeft (LocalVariables|GetLocalSquare)) (Variables|/Game/Blueprints/Structures/BP_Square.BP_Square_C|GetCentreLeft (LocalVariables|GetLocalSquare)))))
    (:8
      ;[1 1 1] Case 8
      (CallFunction|MeshfromPoints (Utilities|Array|MakeArray (Variables|/Game/Blueprints/Structures/BP_Square.BP_Square_C|GetTopLeft (LocalVariables|GetLocalSquare)) (Variables|/Game/Blueprints/Structures/BP_Square.BP_Square_C|GetCentreTop (LocalVariables|GetLocalSquare)) (Variables|/Game/Blueprints/Structures/BP_Square.BP_Square_C|GetCentreLeft (LocalVariables|GetLocalSquare)))))
    (:9
      ;[1 1 1] Case 9
      (CallFunction|MeshfromPoints (Utilities|Array|MakeArray (Variables|/Game/Blueprints/Structures/BP_Square.BP_Square_C|GetTopLeft (LocalVariables|GetLocalSquare)) (Variables|/Game/Blueprints/Structures/BP_Square.BP_Square_C|GetCentreTop (LocalVariables|GetLocalSquare)) (Variables|/Game/Blueprints/Structures/BP_Square.BP_Square_C|GetCentreBottom (LocalVariables|GetLocalSquare)) (Variables|/Game/Blueprints/Structures/BP_Square.BP_Square_C|GetBottomLeft (LocalVariables|GetLocalSquare)))))
    (:10
      ;[1 1 1] Case 10
      (CallFunction|MeshfromPoints (Utilities|Array|MakeArray (Variables|/Game/Blueprints/Structures/BP_Square.BP_Square_C|GetTopLeft (LocalVariables|GetLocalSquare)) (Variables|/Game/Blueprints/Structures/BP_Square.BP_Square_C|GetCentreTop (LocalVariables|GetLocalSquare)) (Variables|/Game/Blueprints/Structures/BP_Square.BP_Square_C|GetCentreRight (LocalVariables|GetLocalSquare)) (Variables|/Game/Blueprints/Structures/BP_Square.BP_Square_C|GetBottomRight (LocalVariables|GetLocalSquare)) (Variables|/Game/Blueprints/Structures/BP_Square.BP_Square_C|GetCentreBottom (LocalVariables|GetLocalSquare)) (Variables|/Game/Blueprints/Structures/BP_Square.BP_Square_C|GetCentreLeft (LocalVariables|GetLocalSquare)))))
    (:11
      ;[1 1 1] Case 11
      (CallFunction|MeshfromPoints (Utilities|Array|MakeArray (Variables|/Game/Blueprints/Structures/BP_Square.BP_Square_C|GetTopLeft (LocalVariables|GetLocalSquare)) (Variables|/Game/Blueprints/Structures/BP_Square.BP_Square_C|GetCentreTop (LocalVariables|GetLocalSquare)) (Variables|/Game/Blueprints/Structures/BP_Square.BP_Square_C|GetCentreRight (LocalVariables|GetLocalSquare)) (Variables|/Game/Blueprints/Structures/BP_Square.BP_Square_C|GetBottomRight (LocalVariables|GetLocalSquare)) (Variables|/Game/Blueprints/Structures/BP_Square.BP_Square_C|GetBottomLeft (LocalVariables|GetLocalSquare)))))
    (:12
      ;[1 1 1] Case 12
      (CallFunction|MeshfromPoints (Utilities|Array|MakeArray (Variables|/Game/Blueprints/Structures/BP_Square.BP_Square_C|GetTopLeft (LocalVariables|GetLocalSquare)) (Variables|/Game/Blueprints/Structures/BP_Square.BP_Square_C|GetTopRight (LocalVariables|GetLocalSquare)) (Variables|/Game/Blueprints/Structures/BP_Square.BP_Square_C|GetCentreRight (LocalVariables|GetLocalSquare)) (Variables|/Game/Blueprints/Structures/BP_Square.BP_Square_C|GetCentreLeft (LocalVariables|GetLocalSquare)))))
    (:13
      ;[1 1 1] Case 13
      (CallFunction|MeshfromPoints (Utilities|Array|MakeArray (Variables|/Game/Blueprints/Structures/BP_Square.BP_Square_C|GetTopLeft (LocalVariables|GetLocalSquare)) (Variables|/Game/Blueprints/Structures/BP_Square.BP_Square_C|GetTopRight (LocalVariables|GetLocalSquare)) (Variables|/Game/Blueprints/Structures/BP_Square.BP_Square_C|GetCentreRight (LocalVariables|GetLocalSquare)) (Variables|/Game/Blueprints/Structures/BP_Square.BP_Square_C|GetCentreBottom (LocalVariables|GetLocalSquare)) (Variables|/Game/Blueprints/Structures/BP_Square.BP_Square_C|GetBottomLeft (LocalVariables|GetLocalSquare)))))
    (:14
      ;[1 1 1] Case 14
      (CallFunction|MeshfromPoints (Utilities|Array|MakeArray (Variables|/Game/Blueprints/Structures/BP_Square.BP_Square_C|GetTopLeft (LocalVariables|GetLocalSquare)) (Variables|/Game/Blueprints/Structures/BP_Square.BP_Square_C|GetTopRight (LocalVariables|GetLocalSquare)) (Variables|/Game/Blueprints/Structures/BP_Square.BP_Square_C|GetBottomRight (LocalVariables|GetLocalSquare)) (Variables|/Game/Blueprints/Structures/BP_Square.BP_Square_C|GetCentreBottom (LocalVariables|GetLocalSquare)) (Variables|/Game/Blueprints/Structures/BP_Square.BP_Square_C|GetCentreLeft (LocalVariables|GetLocalSquare)))))
    (:15
      ;[1 1 1] Case 15
      (CallFunction|MeshfromPoints (Utilities|Array|MakeArray (Variables|/Game/Blueprints/Structures/BP_Square.BP_Square_C|GetTopLeft (LocalVariables|GetLocalSquare)) (Variables|/Game/Blueprints/Structures/BP_Square.BP_Square_C|GetTopRight (LocalVariables|GetLocalSquare)) (Variables|/Game/Blueprints/Structures/BP_Square.BP_Square_C|GetBottomRight (LocalVariables|GetLocalSquare)) (Variables|/Game/Blueprints/Structures/BP_Square.BP_Square_C|GetBottomLeft (LocalVariables|GetLocalSquare))))
      (Utilities|Array|AddUnique _checkedvertices (Variables|/Game/Blueprints/Structures/BP_Node.BP_Node_C|GetVertexIndex (Variables|/Game/Blueprints/Structures/BP_Square.BP_Square_C|GetTopLeft (LocalVariables|GetLocalSquare))))
      (Utilities|Array|AddUnique _checkedvertices (Variables|/Game/Blueprints/Structures/BP_Node.BP_Node_C|GetVertexIndex (Variables|/Game/Blueprints/Structures/BP_Square.BP_Square_C|GetTopRight (LocalVariables|GetLocalSquare))))
      (Utilities|Array|AddUnique _checkedvertices (Variables|/Game/Blueprints/Structures/BP_Node.BP_Node_C|GetVertexIndex (Variables|/Game/Blueprints/Structures/BP_Square.BP_Square_C|GetBottomRight (LocalVariables|GetLocalSquare))))
      (Utilities|Array|AddUnique _checkedvertices (Variables|/Game/Blueprints/Structures/BP_Node.BP_Node_C|GetVertexIndex (Variables|/Game/Blueprints/Structures/BP_Square.BP_Square_C|GetBottomLeft (LocalVariables|GetLocalSquare)))))))

(fn CreateWallMesh
  (bind _wallvertices (LocalVariables|GetWallVertices))
  (bind _walltriangles (LocalVariables|GetWallTriangles))
  (CallFunction|CalculateMeshOutlines)
  (for _array_element (Variables|/Game/Blueprints/Structures/BP_IntMatrix.BP_IntMatrix_C|GetData (Variables|Default|GetOutlines))
    (bind _output_get (LocalVariables|SetOutline (Variables|/Game/Blueprints/Structures/BP_IntList.BP_IntList_C|GetIntList _array_element)))
    (for _index (range 0 (- (Utilities|Array|Length _output_get) 1))
      (LocalVariables|SetI _index)
      (LocalVariables|SetStartIndex (Utilities|Array|Length _wallvertices))
      (Utilities|Array|Add _wallvertices (Utilities|Array|Get(acopy) (Variables|Default|GetVertices) (Utilities|Array|Get(acopy) (LocalVariables|GetOutline) (LocalVariables|GetI))))
      (Utilities|Array|Add _wallvertices (Utilities|Array|Get(acopy) (Variables|Default|GetVertices) (Utilities|Array|Get(acopy) (LocalVariables|GetOutline) (+ (LocalVariables|GetI) 1))))
      (Utilities|Array|Add _wallvertices (- (Utilities|Array|Get(acopy) (Variables|Default|GetVertices) (Utilities|Array|Get(acopy) (LocalVariables|GetOutline) (LocalVariables|GetI))) (* (Math|Vector|MakeVector 0.0 1.0 0.0) (Variables|Default|GetWallHeight))))
      (Utilities|Array|Add _wallvertices (- (Utilities|Array|Get(acopy) (Variables|Default|GetVertices) (Utilities|Array|Get(acopy) (LocalVariables|GetOutline) (+ (LocalVariables|GetI) 1))) (* (Math|Vector|MakeVector 0.0 1.0 0.0) (Variables|Default|GetWallHeight))))
      (Utilities|Array|Add _walltriangles (LocalVariables|GetStartIndex))
      (Utilities|Array|Add _walltriangles (+ (LocalVariables|GetStartIndex) 2))
      (Utilities|Array|Add _walltriangles (+ (LocalVariables|GetStartIndex) 3))
      (Utilities|Array|Add _walltriangles (+ (LocalVariables|GetStartIndex) 3))
      (Utilities|Array|Add _walltriangles (+ (LocalVariables|GetStartIndex) 1))
      (Utilities|Array|Add _walltriangles (LocalVariables|GetStartIndex))))
  (Class|ProceduralMeshComponent|CreateMeshSectionLinearColor (Variables|Default|GetWallMesh) 0 (LocalVariables|GetWallVertices) (LocalVariables|GetWallTriangles) 0 0 0 0 false))

(fn CalculateMeshOutlines
  (bind _outlines (Variables|Default|GetOutlines))
  (for _index (range 0 (- (Utilities|Array|Length (Variables|Default|GetVertices)) 1))
    (bind _output_get (LocalVariables|SetVertexIndex _index))
    (if (not (Utilities|Array|ContainsItem (Variables|Default|GetCheckedVertices) _output_get))
      (bind _connectedoutlinevertex (CallFunction|GetConnectedOutlineVertex _output_get))
      (bind _output_get_2 (LocalVariables|SetNewOutlineVertex _connectedoutlinevertex))
      (if (!= _output_get_2 -1)
        (Utilities|Array|AddUnique (Variables|Default|GetCheckedVertices) (LocalVariables|GetVertexIndex))
        (bind _output_get_3 (LocalVariables|SetNewOutline (Utilities|Array|MakeArray (LocalVariables|GetVertexIndex))))
        (Default|Add (Variables|Default|GetOutlines) _output_get_3)
        (CallFunction|FollowOutline (LocalVariables|GetNewOutlineVertex) (- (Utilities|Array|Length (Variables|/Game/Blueprints/Structures/BP_IntMatrix.BP_IntMatrix_C|GetData (Variables|Default|GetOutlines))) 1))
        (Utilities|Array|Add (Default|GetRow _outlines (- (Utilities|Array|Length (Variables|/Game/Blueprints/Structures/BP_IntMatrix.BP_IntMatrix_C|GetData _outlines)) 1)) (LocalVariables|GetVertexIndex))))))

(fn GetConnectedOutlineVertex
  (params (VertexIndex :type Integer))
  (bind _output_get (LocalVariables|SetLocalVertexIndex VertexIndex))
  (bind _output_get_2 (LocalVariables|SetTrianglesContainingVertex (Default|GetValues (Variables|Default|GetTriangleDictionary) _output_get)))
  (for _array_element _output_get_2
    (bind _output_get_3 (LocalVariables|SetTriangle _array_element))
    (for _index (range 0 2)
      (bind _output_get_4 (LocalVariables|SetVertexB (Default|GetVertex _output_get_3 _index)))
      (if (and (!= _output_get_4 (LocalVariables|GetLocalVertexIndex)) (not (Utilities|Array|ContainsItem (Variables|Default|GetCheckedVertices) (LocalVariables|GetVertexB))))
        (bind _isoutlineedge (CallFunction|IsOutlineEdge (LocalVariables|GetLocalVertexIndex) (LocalVariables|GetVertexB)))
        (if _isoutlineedge
          (return (LocalVariables|GetVertexB))))))
  (return -1))

(fn IsOutlineEdge
  (params (VertexA :type Integer) (VertexB :type Integer))
  (bind _triangledictionary (Variables|Default|GetTriangleDictionary))
  (bind _triangles (Default|GetValues _triangledictionary VertexA))
  (LocalVariables|SetLocalVertexB VertexB)
  (LocalVariables|SetSharedTriangleCount 0)
  (bind _output_get (LocalVariables|SetTrianglesContainingVertexA _triangles))
  (bind _index (Utilities|FlowControl|ForLoopwithBreak 0 (- (Utilities|Array|Length _triangles) 1) :!label _label)
    (:LoopBody
      (if (Default|Contains (Utilities|Array|Get(acopy) _output_get _index) (LocalVariables|GetLocalVertexB))
        (bind _result (Math|Integer|IncrementInt (LocalVariables|GetSharedTriangleCount))
          (:%20%20
            (if (> _result 1)
              (goto _label Break))))))
    (:Completed
      (return (== (LocalVariables|GetSharedTriangleCount) 1)))))

(fn FollowOutline
  (params (VertexIndex :type Integer) (OutlineIndex :type Integer))
  (LocalVariables|SetLocalVertexIndex VertexIndex)
  (bind _output_get (LocalVariables|SetLocalOutlineIndex OutlineIndex))
  (Utilities|Array|Add (Default|GetRow (Variables|Default|GetOutlines) _output_get) (LocalVariables|GetLocalVertexIndex))
  (Utilities|Array|AddUnique (Variables|Default|GetCheckedVertices) (LocalVariables|GetLocalVertexIndex))
  (bind _connectedoutlinevertex (CallFunction|GetConnectedOutlineVertex (LocalVariables|GetLocalVertexIndex)))
  (bind _output_get_2 (LocalVariables|SetNextVertexIndex _connectedoutlinevertex))
  (if (!= _output_get_2 -1)
    (CallFunction|FollowOutline (LocalVariables|GetNextVertexIndex) (LocalVariables|GetLocalOutlineIndex))))