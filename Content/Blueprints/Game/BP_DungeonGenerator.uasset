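; BP_DungeonGenerator builds a cave-style dungeon layout using cellular automata.
; GenerateMap randomly fills a BP_IntMatrix with walls and floor from a random stream and fill percentage, forcing walls on the edges.
; Smoothing passes then set each cell by its eight-neighbour wall count, updating the grid in place.
; The map gets a solid border and goes to a spawned BP_MeshGenerator for meshing; an instanced debug-tile view exists but is disconnected.
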(fn ConstructionScript)

(fn GenerateMap
  (bind _returnvalue (Game|ConstructObjectfromClass "/Game/Blueprints/Structures/BP_IntMatrix.BP_IntMatrix_C" self))
  (bind _output_get (Variables|Default|SetMap _returnvalue))
  (Default|Init _output_get (Variables|Default|GetWidth) (Variables|Default|GetHeight))
  (CallFunction|RandomFillMap)
  (CallFunction|SmoothMap)
  (bind _borderedmap (CallFunction|CreateBorderedMap))
  (Variables|Default|SetBorderedMap _borderedmap)
  (bind _returnvalue_2 (Game|SpawnActorfromClass "/Game/Blueprints/Game/BP_MeshGenerator.BP_MeshGenerator_C" (Transformation|GetActorTransform) "Undefined" 0 0))
  (Default|GenerateMesh _returnvalue_2 (Variables|Default|GetBorderedMap) (Variables|Default|GetTileSize)))

(fn RandomFillMap
  (for _index (range 0 (- (Variables|Default|GetWidth) 1))
    (LocalVariables|SetX _index)
    (for _index_2 (range 0 (- (Variables|Default|GetHeight) 1))
      (LocalVariables|SetY _index_2)
      (if (Math|Boolean|ORBoolean (== (LocalVariables|GetX) 0) (== (LocalVariables|GetX) (- (Variables|Default|GetWidth) 1)) (== (LocalVariables|GetY) 0) (== (LocalVariables|GetY) (- (Variables|Default|GetHeight) 1)))
        (Default|SetElement (Variables|Default|GetMap) (LocalVariables|GetX) (LocalVariables|GetY) 1 :!label _label)
        (else
          ;[1 1 1] Check if should put a wall or tile based on the fill percentage
          (if (< (Math|Random|RandomIntegerinRangefromStream 0 100 (Variables|Default|GetRandomStream)) (Variables|Default|GetFillPercentage))
            (goto _label)
            (else
              (Default|SetElement (Variables|Default|GetMap) (LocalVariables|GetX) (LocalVariables|GetY)))))))))

(fn CreateDebugTiles
  (params (Map :type BP%20Int%20Matrix%20Object%20Reference))
  (bind _output_get (LocalVariables|SetLocalMap Map))
  (LocalVariables|SetLocalMapWidth (Default|GetNumRows _output_get))
  (LocalVariables|SetLocalMapHeight (Default|GetNumCols _output_get))
  (for _index (range 0 (- (LocalVariables|GetLocalMapWidth) 1))
    (LocalVariables|SetX _index)
    (for _index_2 (range 0 (- (LocalVariables|GetLocalMapHeight) 1))
      (LocalVariables|SetY _index_2)
      (switch int (Default|GetElement (LocalVariables|GetLocalMap) (LocalVariables|GetX) (LocalVariables|GetY))
        (:0
          (Components|InstancedStaticMesh|AddInstance (Variables|Default|GetEmpty) (Math|Conversions|ToTransform(Vector) (+ (Math|Vector|MakeVector (Math|Conversions|ToFloat(Integer) (* (LocalVariables|GetX) (Variables|Default|GetTileSize))) (Math|Conversions|ToFloat(Integer) (* (LocalVariables|GetY) (Variables|Default|GetTileSize))) 0.0) (Transformation|GetActorLocation)))))
        (:1
          (Components|InstancedStaticMesh|AddInstance (Variables|Default|GetFilled) (Math|Conversions|ToTransform(Vector) (+ (Math|Vector|MakeVector (Math|Conversions|ToFloat(Integer) (* (LocalVariables|GetX) (Variables|Default|GetTileSize))) (Math|Conversions|ToFloat(Integer) (* (LocalVariables|GetY) (Variables|Default|GetTileSize))) 0.0) (Transformation|GetActorLocation)))))))))

(fn SmoothMap
  (for _index (range 0 (Variables|Default|GetSmoothnessLevel))
    (for _index_2 (range 0 (- (Variables|Default|GetWidth) 1))
      (LocalVariables|SetX _index_2)
      (for _index_3 (range 0 (- (Variables|Default|GetHeight) 1))
        (LocalVariables|SetY _index_3)
        (bind _walls (CallFunction|GetSurroundingWallCount (LocalVariables|GetX) (LocalVariables|GetY)))
        (bind _output_get (LocalVariables|SetNeighbourWallTiles _walls))
        (if (> _output_get 4)
          (Default|SetElement (Variables|Default|GetMap) (LocalVariables|GetX) (LocalVariables|GetY) 1)
          (elif (< _output_get 4)
            (Default|SetElement (Variables|Default|GetMap) (LocalVariables|GetX) (LocalVariables|GetY))))))))

(fn GetSurroundingWallCount
  (params (GridX :type Integer) (GridY :type Integer))
  (LocalVariables|SetLocalGridX GridX)
  (LocalVariables|SetLocalGridY GridY)
  (LocalVariables|SetWallCount 0)
  (for _index (range (- (LocalVariables|GetLocalGridX) 1) (+ (LocalVariables|GetLocalGridX) 1))
    (LocalVariables|SetNeighbourX _index)
    (for _index_2 (range (- (LocalVariables|GetLocalGridY) 1) (+ (LocalVariables|GetLocalGridY) 1))
      (LocalVariables|SetNeighbourY _index_2)
      (if (Math|Boolean|ANDBoolean (>= (LocalVariables|GetNeighbourX) 0) (< (LocalVariables|GetNeighbourX) (Variables|Default|GetWidth)) (>= (LocalVariables|GetNeighbourY) 0) (< (LocalVariables|GetNeighbourY) (Variables|Default|GetHeight)))
        (if (or (!= (LocalVariables|GetNeighbourX) (LocalVariables|GetLocalGridX)) (!= (LocalVariables|GetNeighbourY) (LocalVariables|GetLocalGridY)))
          (LocalVariables|SetWallCount (+ (LocalVariables|GetWallCount) (Default|GetElement (Variables|Default|GetMap) (LocalVariables|GetNeighbourX) (LocalVariables|GetNeighbourY)))))
        (else
          (Math|Integer|IncrementInt (LocalVariables|GetWallCount))))))
  (return (LocalVariables|GetWallCount)))

(fn CreateBorderedMap
  (bind _bordersize (Variables|Default|GetBorderSize))
  (bind _bordersize_2 (Variables|Default|GetBorderSize))
  (bind _returnvalue (* _bordersize_2 2))
  (LocalVariables|SetBorderedMapWidth (+ (Variables|Default|GetWidth) _returnvalue))
  (LocalVariables|SetBorderedMapHeight (+ (Variables|Default|GetHeight) _returnvalue))
  (bind _returnvalue_2 (Game|ConstructObjectfromClass "/Game/Blueprints/Structures/BP_IntMatrix.BP_IntMatrix_C" self))
  (bind _intmatrix (Default|Init _returnvalue_2 (LocalVariables|GetBorderedMapWidth) (LocalVariables|GetBorderedMapHeight)))
  (for _index (range 0 (- (LocalVariables|GetBorderedMapWidth) 1))
    (LocalVariables|SetX _index)
    (for _index_2 (range 0 (- (LocalVariables|GetBorderedMapHeight) 1))
      (LocalVariables|SetY _index_2)
      (if (Math|Boolean|ANDBoolean (>= (LocalVariables|GetX) (Variables|Default|GetBorderSize)) (< (LocalVariables|GetX) (+ (Variables|Default|GetWidth) (Variables|Default|GetBorderSize))) (>= (LocalVariables|GetY) (Variables|Default|GetBorderSize)) (< (LocalVariables|GetY) (+ (Variables|Default|GetHeight) (Variables|Default|GetBorderSize))))
        (Default|SetElement _intmatrix (LocalVariables|GetX) (LocalVariables|GetY) (Default|GetElement (Variables|Default|GetMap) (- (LocalVariables|GetX) _bordersize) (- (LocalVariables|GetY) _bordersize)))
        (else
          (Default|SetElement _intmatrix (LocalVariables|GetX) (LocalVariables|GetY) 1)))))
  (return _intmatrix))